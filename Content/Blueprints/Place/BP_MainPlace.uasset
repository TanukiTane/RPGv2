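; BP_MainPlace is a place actor that tracks an NPC using it and can rotate that NPC.
; Start stores the given character as the NPC and marks the place active, while Stop only clears the active flag.
; While active, Rotation adds the passed Place's root world rotation to the NPC's current rotation as an offset, rather than setting it.
; Tick and the construction script are empty.
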(event `self.ReceiveTick`
  (params (DeltaSeconds :type "Float (single-precision)")))

(fn `-Rotation`
  (params (Place :type "/Game/Blueprints/Place/BP_MainPlace Object Reference"))
  (if (`self.PlaceActive`)
    (`self.K2_AddActorWorldRotation` (`self.NPC`) (`SceneComponent.K2_GetComponentRotation` (`Actor.RootComponent` Place)) false false)))

(fn `-Start`
  (params (Chatacter :type "/Game/Blueprints/BP_MainChacter Object Reference"))
  (set `self.NPC` Chatacter)
  (set `self.PlaceActive` true))

(fn `-Stop`
  (params (Chatacter :type "/Game/Blueprints/BP_MainChacter Object Reference"))
  (set `self.PlaceActive` false))

(fn `UserConstructionScript`)