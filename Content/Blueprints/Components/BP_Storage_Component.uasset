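; Character storage component that holds picked-up weapons and ammo, and handles equipping, holstering and dropping weapons.
; ItemsAllAdd routes bullets into stacks merged by class and weapons into rifle or gun slots, dropping the one replaced.
; Weapons move between hand and holster sockets, with the attach event using delays to briefly stop the character.
; Swaps holster the current weapon, then poll by timer until the character's animation ends before drawing the next.
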(event `self.-Init`
  ;[1 1 1] Init
  (`parent.-Init`))

(event `Weapon Attach`
  (params (Weapon :type "/Game/Blueprints/Storage/Weapon/BP_WeaponActor Object Reference") (SocketName :type Name))
  ;[1 1 1] Weapon Attach
  (`|ExecutionSequence`
    (:`then_0`
      (set `/Game/Blueprints/BP_MainChacter.IsStopped` true (`self.Character`))
      (`KismetSystemLibrary.Delay` 0.7)
      (`self.WeaponAttach` Weapon SocketName))
    (:`then_1`
      (`KismetSystemLibrary.Delay` 1.8)
      (set `/Game/Blueprints/BP_MainChacter.IsStopped` false (`self.Character`)))
    (:`then_2`
      (if (== SocketName "Skt_CurWeapon")
        (set `/Game/Blueprints/BP_MainChacter.IsCurWeapon` true (`self.Character`))
        (else
          (set `/Game/Blueprints/BP_MainChacter.IsCurWeapon` false (`self.Character`)))))))

(fn `- Find Cur Bullet`
  (returns (Bullets :type "/Game/Blueprints/Storage/Bullets/BP_St_Act_Bullet Object Reference"))
  (locals (L_Bullets :type "/Game/Blueprints/Storage/Bullets/BP_St_Act_Bullet Object Reference"))
  (bind _weaponcurrent (`self.WeaponCurrent`)
    (:`then`
      (bind _asbp_weapon_fire_actor (cast `/Game/Blueprints/Storage/Weapon/Fire/BP_WeaponFireActor` _weaponcurrent)
        (:`then`
          (for _array_element (`self.ItemsBullets`)
            (if (== (`GameplayStatics.GetObjectClass` _array_element) (`/Game/Blueprints/Storage/Weapon/Fire/BP_WeaponFireActor.Bullets_Type_Fire` _asbp_weapon_fire_actor))
              (set `local.L_Bullets` _array_element)
              (break)))
          (bind _l_bullets (`local.L_Bullets`)
            (:`then`
              (return _l_bullets))
            (:`else`
              (return null))))
        (:`CastFailed`
          _)))
    (:`else`
      _))
  (return null))

(fn `-AttachToWeapon`
  (params (ActorWeapon :type "/Game/Blueprints/Storage/Weapon/Fire/BP_WeaponFireActor Object Reference") (L_CurWeaponActive :type "/Game/Blueprints/Storage/Weapon/Fire/BP_WeaponFireActor Object Reference") (LCurWeapon :type "/Game/Blueprints/Storage/Weapon/BP_WeaponActor Object Reference") (SocketName :type Name))
  (`PrimitiveComponent.SetSimulatePhysics` (`/Game/Blueprints/Storage/BP_StorageActor.StaticMesh` ActorWeapon) false)
  (`Actor.SetActorEnableCollision` ActorWeapon false)
  (`Actor.K2_SetActorLocation` ActorWeapon (0.0 0.0 0.0) false false)
  (`Actor.K2_SetActorRotation` :`self` ActorWeapon)
  (if (and (== L_CurWeaponActive LCurWeapon) (!= LCurWeapon null))
    (`self.WeaponAttach` null "Skt_CurWeapon")
    (set `self.WeaponCurrent` ActorWeapon)
    (else
      (`self.WeaponAttach` ActorWeapon SocketName))))

(fn `-ItemsAllAdd`
  (params (ItemsAdd :type "/Game/Blueprints/Storage/BP_StorageActor Object Reference"))
  (locals (l_ItemsAdd :type "/Game/Blueprints/Storage/BP_StorageActor Object Reference"))
  (bind _output_get (set `local.l_ItemsAdd` ItemsAdd))
  (bind _asbp_st_act_bullet (cast `/Game/Blueprints/Storage/Bullets/BP_St_Act_Bullet` _output_get)
    (:`then`
      (`Actor.SetOwner` _asbp_st_act_bullet (`self.Character`))
      (`self.-ItemWeaponBulletsAdd` _asbp_st_act_bullet))
    (:`CastFailed`
      (bind _asbp_weapon_actor (cast `/Game/Blueprints/Storage/Weapon/BP_WeaponActor` (`local.l_ItemsAdd`)))
      (`Actor.SetOwner` _asbp_weapon_actor (`self.Character`))
      (`self.WeaponAdd` _asbp_weapon_actor))))

(fn `-ItemWeaponAdd`
  (params (ItemWeaponAdd :type "/Game/Blueprints/Storage/BP_StorageActor Object Reference (by ref)"))
  (`KismetArrayLibrary.Array_Add` (`self.ItemsWeapon`) ItemWeaponAdd))

(fn `-ItemWeaponBulletsAdd`
  (params (ItemBulletsAdd :type "/Game/Blueprints/Storage/Bullets/BP_St_Act_Bullet Object Reference (by ref)"))
  (locals (L_BulletsAdd :type "/Game/Blueprints/Storage/Bullets/BP_St_Act_Bullet Object Reference") (L_FindBullet :type "/Game/Blueprints/Storage/Bullets/BP_St_Act_Bullet Object Reference"))
  (set `local.L_BulletsAdd` ItemBulletsAdd)
  (for _array_element (`self.ItemsBullets`)
    (if (== (`GameplayStatics.GetObjectClass` _array_element) (`GameplayStatics.GetObjectClass` (`local.L_BulletsAdd`)))
      (set `local.L_FindBullet` _array_element)
      (break)))
  (`local.L_FindBullet`
    (:`then`
      (set `/Game/Blueprints/Storage/Bullets/BP_St_Act_Bullet.Value` (+ (`/Game/Blueprints/Storage/Bullets/BP_St_Act_Bullet.Value` (`local.L_BulletsAdd`)) (`/Game/Blueprints/Storage/Bullets/BP_St_Act_Bullet.Value` (`local.L_FindBullet`))) (`local.L_FindBullet`))
      (`Actor.K2_DestroyActor` (`local.L_BulletsAdd`)))
    (:`else`
      (`KismetArrayLibrary.Array_Add` (`self.ItemsBullets`) (`local.L_BulletsAdd`))
      (`Actor.SetActorEnableCollision` (`local.L_BulletsAdd`) false)
      (`Actor.K2_SetActorLocation` (`local.L_BulletsAdd`) (0.0 0.0 0.0) false false)
      (`Actor.SetActorHiddenInGame` (`local.L_BulletsAdd`) false))))

(fn `-WeaponChangeDelay`
  (if (`/Game/Blueprints/BP_MainChacter.IsPlayingAnimation` (`self.Character`))
    (`KismetSystemLibrary.K2_SetTimer` null "-WeaponChangeDelay" 0.1)
    (else
      (bind _tempweaponcur (`self.TempWeaponCur`)
        (:`then`
          (`self.WeaponChange` _tempweaponcur))
        (:`else`)))))

(fn `WeaponAdd`
  (params (Weapon :type "/Game/Blueprints/Storage/Weapon/BP_WeaponActor Object Reference"))
  (locals (L_CurrRiffle :type "/Game/Blueprints/Storage/Weapon/Fire/Rifle/BP_WeaponRifleActor Object Reference") (L_CurrWeapon :type "/Game/Blueprints/Storage/Weapon/BP_WeaponActor Object Reference") (L_CurGun :type "/Game/Blueprints/Storage/Weapon/Fire/Gun/BP_Weapon_Fire_GunActor Object Reference"))
  (bind _asbp_weapon_fire_actor (cast `/Game/Blueprints/Storage/Weapon/Fire/BP_WeaponFireActor` Weapon))
  (bind _asbp_weapon_rifle_actor (cast `/Game/Blueprints/Storage/Weapon/Fire/Rifle/BP_WeaponRifleActor` _asbp_weapon_fire_actor)
    (:`then`
      (bind _weaponrifle (`self.WeaponRifle`)
        (:`then`
          ;[1 1 1] Выбросить и добавить новую
          (set `local.L_CurrRiffle` _weaponrifle)
          (set `local.L_CurrWeapon` (`self.WeaponCurrent`))
          (`self.WeaponDrop` _weaponrifle))
        (:`else`
          _))
      (bind _output_get (set `self.WeaponRifle` _asbp_weapon_rifle_actor))
      (`self.-AttachToWeapon` _output_get (`local.L_CurrRiffle`) (`local.L_CurrWeapon`) "Skt_HideRifle"))
    (:`CastFailed`
      (bind _asbp_weapon_fire_gun_actor (cast `/Game/Blueprints/Storage/Weapon/Fire/Gun/BP_Weapon_Fire_GunActor` _asbp_weapon_fire_actor))
      (bind _weapongun (`self.WeaponGun`)
        (:`then`
          (set `local.L_CurGun` _asbp_weapon_fire_gun_actor)
          (set `local.L_CurrWeapon` (`self.WeaponCurrent`))
          (`self.WeaponDrop` _weapongun))
        (:`else`
          _))
      (bind _output_get_2 (set `self.WeaponGun` _asbp_weapon_fire_gun_actor))
      (`self.-AttachToWeapon` _output_get_2 (`local.L_CurGun`) (`local.L_CurrWeapon`) "Skt_HideRifle"))))

(fn `WeaponAttach`
  (params (Weapon :type "/Game/Blueprints/Storage/Weapon/BP_WeaponActor Object Reference") (SocketName :type Name))
  (`Actor.K2_AttachToComponent` Weapon (`Character.Mesh` (`self.Character`)) SocketName "KeepRelative" "KeepRelative" "KeepRelative" true))

(fn `WeaponChange`
  (params (Weapon :type "/Game/Blueprints/Storage/Weapon/BP_WeaponActor Object Reference"))
  (locals (L_Input_Weapon :type "/Game/Blueprints/Storage/Weapon/BP_WeaponActor Object Reference"))
  (set `local.L_Input_Weapon` Weapon)
  (`/Engine/EditorBlueprintResources/StandardMacros.IsValid` (`local.L_Input_Weapon`)
    (:`Is Valid`
      (if (not (`/Game/Blueprints/BP_MainChacter.IsPlayingAnimation` (`self.Character`)))
        (if (== (`local.L_Input_Weapon`) (`self.WeaponCurrent`))
          ;[1 1 1] Снять оружие
          (set `self.WeaponCurrent` null)
          (`self.Weapon Attach` (`local.L_Input_Weapon`) "Skt_HideRifle")
          (else
            (bind _weaponcurrent (`self.WeaponCurrent`)
              (:`then`
                ;[1 1 1] Взять оружие
                (`self.WeaponChange` _weaponcurrent)
                (set `self.TempWeaponCur` (`local.L_Input_Weapon`))
                (`KismetSystemLibrary.K2_SetTimer` null "-WeaponChangeDelay" 0.1))
              (:`else`
                (bind _output_get (set `self.WeaponCurrent` (`local.L_Input_Weapon`)))
                (`self.Weapon Attach` _output_get "Skt_CurWeapon")))))
        (else
          (set `self.TempWeaponCur` (`local.L_Input_Weapon`)))))))

(fn `WeaponDrop`
  (params (Weapon :type "/Game/Blueprints/Storage/Weapon/BP_WeaponActor Object Reference"))
  (bind _character (`self.Character`))
  (bind _staticmesh (`/Game/Blueprints/Storage/BP_StorageActor.StaticMesh` Weapon))
  (`PrimitiveComponent.SetSimulatePhysics` _staticmesh true)
  (`SceneComponent.K2_DetachFromComponent` _staticmesh "KeepRelative" "KeepRelative" "KeepRelative" true)
  (`Actor.SetActorEnableCollision` Weapon true)
  (`Actor.SetOwner` Weapon null)
  (if (== (`self.WeaponCurrent`) Weapon)
    (set `self.WeaponCurrent` null))
  (`Actor.K2_SetActorLocation` Weapon (+ (`Actor.K2_GetActorLocation` _character) (* (`Actor.GetActorForwardVector` _character) 100.0)) false false)
  (if (== (`self.WeaponRifle`) Weapon)
    (set `self.WeaponRifle` null)))