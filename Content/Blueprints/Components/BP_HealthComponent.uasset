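; BP_HealthComponent is a component that tracks a character's health and triggers death when it runs out.
; Its Init event only calls the parent implementation.
; HealthChange adds an incoming value to Health, clamps it to zero once it drops to or below zero, and then calls IsDeath on the Character.
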(event `self.-Init`
  ;[1 1 1] Init
  (`parent.-Init`))

(fn `-Health Change`
  (params (Health :type "Float (double-precision)"))
  (set `self.Health` (+ Health (`self.Health`)))
  (if (<= (`self.Health`) 0.0)
    ;[1 1 1] Set Death = 0
    (set `self.Health` 0.0)
    (`/Game/Blueprints/BP_MainChacter.-IsDeath` (`self.Character`))))