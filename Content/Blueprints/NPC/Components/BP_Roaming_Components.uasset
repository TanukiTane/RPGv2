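; NPC roaming component that moves the character between destinations through its AI controller and stops when the NPC dies.
; With a NavMesh, it cycles through the NPC's Place actors or picks random reachable points, triggering the Place on arrival and waiting its delay before moving on.
; Without a NavMesh, it walks the NPC back to its initial location and restores its rotation.
; Function-name timers drive movement, distance polling and waits.
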(event `self.-Init`
  ;[1 1 1] init
  (`parent.-Init`)
  (`/Engine/EditorBlueprintResources/StandardMacros.IsValid` (`/Game/Blueprints/NPC/BP_NPC_Character.NavMesh` (`self.NPC`))
    (:`Is Not Valid`
      (set `self.Location` (`Actor.K2_GetActorLocation` (`self.NPC`)))
      (set `self.Rotation` (`Actor.K2_GetActorRotation` (`self.NPC`))))))

(event `self.-Start`
  ;[1 1 1] Start
  (`/Engine/EditorBlueprintResources/StandardMacros.IsValid` (`/Game/Blueprints/NPC/BP_NPC_Character.NavMesh` (`self.NPC`))
    (:`Is Valid`
      (`parent.-Start`)
      (`self.-GoToNewTarget`))
    (:`Is Not Valid`
      (`parent.-Start`)
      (`self.-GoToTarget`)))
  (set `self.Roaming` true))

(event `self.-Stop`
  ;[1 1 1] Stop
  (`parent.-Stop`)
  (`KismetSystemLibrary.K2_ClearAndInvalidateTimerHandle` (`self.Timer -GoToTarget2`))
  (`KismetSystemLibrary.K2_ClearAndInvalidateTimerHandle` (`self.Timer-GoToTarget`))
  (`KismetSystemLibrary.K2_ClearAndInvalidateTimerHandle` (`self.Timer-GoToNewTarget`))
  (set `self.Roaming` false)
  (set `self.Moving` false)
  (set `self.Waiting` false)
  ;[1 1 1] Stop Movement
  (`MovementComponent.StopMovementImmediately` (`Character.CharacterMovement` (`self.NPC`)))
  ;[1 1 1] SetLocation
  (`/Engine/EditorBlueprintResources/StandardMacros.IsValid` (`/Game/Blueprints/NPC/BP_NPC_Character.NavMesh` (`self.NPC`))
    (:`Is Valid`
      (set `self.Location` (0.0 0.0 0.0)))))

(event `self.ReceiveTick`
  (params (DeltaSeconds :type "Float (single-precision)"))
  ;[1 1 1] Stop component if NPC dead
  (if (`/Game/Blueprints/BP_MainChacter.isDeath` (`self.NPC`))
    (if (`self.Roaming`)
      (`self.-Stop`))))

(fn `-Find location`
  (returns (RandomLocation :type "Vector Structure"))
  (locals (L_LocaltionPlace :type "Vector Structure" :default (0.0 0.0 0.0)))
  (bind _npc (`self.NPC`))
  (bind (_randomlocation _returnvalue) (`NavigationSystemV1.K2_GetRandomReachablePointInRadius` (`Actor.K2_GetActorLocation` (`self.NPC`)) (`self.RadiusFindPoint`) (`/Game/Blueprints/NPC/BP_NPC_Character.NavMesh` (`self.NPC`)) null))
  (set `self.LengthArr` (`KismetArrayLibrary.Array_Length` (`/Game/Blueprints/NPC/BP_NPC_Character.Place` (`self.NPC`))))
  (if (`self.ModePlace`)
    (if (> (`self.LengthArr`) 0)
      (if (>= (`self.CurPlace`) (`self.LengthArr`))
        (set `self.CurPlace` 0))
      (set `self.Place` (`|GetArrayItem` (`/Game/Blueprints/NPC/BP_NPC_Character.Place` (`self.NPC`)) (`self.CurPlace`)))
      (set `self.LengthPlace` (`/Game/Blueprints/Place/BP_MainPlace.LengthPlace` (`self.Place`)))
      (set `self.DelayStopGoToTarget` (`/Game/Blueprints/Place/BP_MainPlace.DelayPlaceWait` (`self.Place`)))
      (if (not (== (`GameplayStatics.GetObjectClass` (`self.Place`)) "/Game/Blueprints/Place/BP_Place_RandomLocation.BP_Place_RandomLocation_C"))
        (set `local.L_LocaltionPlace` (`Actor.K2_GetActorLocation` (`self.Place`)))
        (`/Engine/EditorBlueprintResources/StandardMacros.IncrementInt` (`self.CurPlace`)
          (:`  `
            (return (`local.L_LocaltionPlace`))))
        (else
          (`/Engine/EditorBlueprintResources/StandardMacros.IncrementInt` (`self.CurPlace`)
            (:`  `
              _))))))
  ;[1 1 1] Random Target
  (if _returnvalue
    (return _randomlocation)
    (else
      (return (+ (`Actor.K2_GetActorLocation` _npc) (* (`Actor.GetActorForwardVector` _npc) 500.0))))))

(fn `-GoToNewTarget`
  (bind _randomlocation (`self.-Find location`))
  (set `self.Location` _randomlocation)
  (set `self.Moving` true)
  (set `self.Waiting` false)
  (bind _returnvalue (`KismetSystemLibrary.K2_SetTimer` null "-GoToTarget" 0.5 true))
  (set `self.Timer-GoToTarget` _returnvalue))

(fn `-GoToTarget`
  (`AIController.MoveToLocation` (`self.NPC_AIController`) (`self.Location`) 50.0 true true false true null true)
  (bind _returnvalue (`KismetSystemLibrary.K2_SetTimer` null "-GoToTarget" 0.1))
  (set `self.Timer -GoToTarget2` _returnvalue)
  (`/Game/Blueprints/NPC/BP_NPC_Character.NavMesh` (`self.NPC`)
    (:`then`
      (if (<= (`self.-VectorLength`) (`self.LengthPlace`))
        (`self.-TargetReached` :!label _label)))
    (:`else`
      (if (<= (`self.-VectorLength`) 100.0)
        (goto _label)))))

(fn `-TargetReached`
  (`/Engine/EditorBlueprintResources/StandardMacros.IsValid` (`/Game/Blueprints/NPC/BP_NPC_Character.NavMesh` (`self.NPC`))
    (:`Is Valid`
      (`MovementComponent.StopMovementImmediately` (`Character.CharacterMovement` (`self.NPC`)))
      (`KismetSystemLibrary.K2_ClearAndInvalidateTimerHandle` (`self.Timer-GoToTarget`))
      (set `self.Location` (0.0 0.0 0.0))
      (set `self.Moving` false)
      (set `self.Waiting` true)
      (`/Game/Blueprints/Place/BP_MainPlace.-Start` (`self.Place`) (`self.NPC`))
      (bind _returnvalue (`KismetSystemLibrary.K2_SetTimer` null "-GoToNewTarget" (`self.DelayStopGoToTarget`)))
      (set `self.Timer-GoToNewTarget` _returnvalue)
      (`KismetSystemLibrary.K2_ClearAndInvalidateTimerHandle` (`self.Timer -GoToTarget2`)))
    (:`Is Not Valid`
      (`MovementComponent.StopMovementImmediately` (`Character.CharacterMovement` (`self.NPC`)))
      (`Actor.K2_SetActorRotation` (`self.NPC`) (`self.Rotation`) false)
      (`KismetSystemLibrary.K2_ClearAndInvalidateTimerHandle` (`self.Timer-GoToTarget`))
      (set `self.Moving` false)
      (set `self.Waiting` true)
      (`KismetSystemLibrary.K2_ClearAndInvalidateTimerHandle` (`self.Timer -GoToTarget2`)))))

(fn `-VectorLength`
  (returns (ReturnValue :type "Float (double-precision)"))
  (return (`KismetMathLibrary.VSize` (- (`Actor.K2_GetActorLocation` (`self.NPC`)) (`self.Location`)))))