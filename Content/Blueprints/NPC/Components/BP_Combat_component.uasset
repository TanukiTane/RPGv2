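; NPC combat component that makes the NPC attack the player target supplied by its AI controller.
; Timer-polled functions use a visibility line trace to turn and fire while the target is seen, or move to its last known location.
; On arrival it waits a delay from the NPC's data before handing off to patrol.
; Tick updates the weapon aim point and stops combat when the NPC dies.
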(event `self.-Init`
  ;[1 1 1] Init
  (`parent.-Init`))

(event `self.-Start`
  ;[1 1 1] Start
  (`parent.-Start`)
  (set `self.IsCombat` true)
  (if (not (`/Game/Blueprints/BP_MainChacter.isDeath` (`self.NPC`)))
    (bind _goalplayer (`/Game/Blueprints/NPC/BP_NPC_AIController.GoalPlayer` (`self.NPC_AIController`))
      (:`then`
        (set `self.Goal Player` _goalplayer)
        (`self.-TurnToGoal`)
        (`self.-FindGoal`))
      (:`else`
        ;[1 1 1] Stop
        (`parent.-Stop` :!label _label)
        (`|ExecutionSequence`
          (:`then_0`
            (set `self.IsCombat` false)
            (set `self.IsOnDo` false)
            (set `self.IsComplited -DelayBeforeCloserComponent` false))
          (:`then_1`
            (`KismetSystemLibrary.K2_ClearAndInvalidateTimerHandle` (`self.Timer -DelayBeforeCloserComponent`))
            (`KismetSystemLibrary.K2_ClearAndInvalidateTimerHandle` (`self.Timer -MoveToLocation`))
            (`KismetSystemLibrary.K2_ClearAndInvalidateTimerHandle` (`self.Timer -IsAttacking`))
            (set `/Game/Blueprints/BP_MainChacter.IsFire` false (`self.NPC`)))
          (:`then_2`
            (set `self.DelayFindTarget` 0.0)))))
    (else
      (goto _label))))

(event `self.-Stop`
  ;[1 1 1] Stop
  (goto _label))

(event `self.ReceiveTick`
  (params (DeltaSeconds :type "Float (single-precision)"))
  (if (`/Game/Blueprints/BP_MainChacter.isDeath` (`self.NPC`))
    (if (`self.IsCombat`)
      (`self.-Stop`))
    (else
      (`|ExecutionSequence`
        (:`then_0`
          (bind _goal_player (`self.Goal Player`)
            (:`then`
              (`/Engine/EditorBlueprintResources/StandardMacros.IsValid` _goal_player
                (:`Is Valid`
                  (set `/Game/Blueprints/BP_MainChacter.WeaponTargetLocation` (`Actor.K2_GetActorLocation` _goal_player) (`self.NPC`)))))
            (:`else`)))))))

(fn `-DelayBeforeCloserComponent`
  (set `self.IsComplited -DelayBeforeCloserComponent` true))

(fn `-FindGoal`
  (set `self.IsAttacking` false)
  (if (`self.-SeeTheGoalNow`)
    (`self.-TurnToGoal`)
    (`|ExecutionSequence`
      (:`then_0`
        ;[1 1 1] Clear logic to begin patrol component
        (if (`self.IsOnDo`)
          (set `self.IsOnDo` false)
          (set `self.IsComplited -DelayBeforeCloserComponent` false)
          (`KismetSystemLibrary.K2_ClearAndInvalidateTimerHandle` (`self.Timer -DelayBeforeCloserComponent`))
          (`/Game/Blueprints/NPC/BP_NPC_Character.Stop_UpdateTimeLine` (`self.NPC`))))
      (:`then_1`
        (if (`/Game/Blueprints/NPC/BP_NPC_Character.isAttackAllowed` (`self.NPC`))
          (`self.-IsAttacking`)
          (else
            (`KismetSystemLibrary.K2_SetTimer` null "-FindGoal" 0.1)))))
    (elif (<= (`KismetMathLibrary.VSize` (- (`Actor.K2_GetActorLocation` (`self.NPC`)) (`self.LocationGoal`))) 100.0)
      (if (not (`self.IsComplited -DelayBeforeCloserComponent`))
        ;[1 1 1] Timer logic of Combat component
        (`KismetSystemLibrary.K2_SetTimer` null "-FindGoal" 0.1)
        (if (not (`self.IsOnDo`))
          (set `self.IsOnDo` true)
          (bind _returnvalue (`KismetSystemLibrary.K2_SetTimer` null "-DelayBeforeCloserComponent" (`.MaxTime_10_1960ECC64E9645FCC4B11B9CF212DC4F` (break `/Game/Data/Struct/ST_DataComponent` (`/Game/Blueprints/NPC/BP_NPC_Character.DataComp` (`self.NPC`))))))
          (set `self.Timer -DelayBeforeCloserComponent` _returnvalue)
          (`/Game/Blueprints/NPC/BP_NPC_Character.UpdateTimeline` (`self.NPC`) true))
        (else
          ;[1 1 1] Call Patrol component
          (`/Game/Blueprints/NPC/BP_NPC_AIController.-Patrol` (`self.NPC_AIController`))))
      (else
        (`KismetSystemLibrary.K2_SetTimer` null "-MoveToLocation" 0.1)))))

(fn `-IsAttacking`
  (if (`self.-SeeTheGoalNow`)
    (set `self.IsAttacking` true)
    (`self.-TurnToGoal`)
    (bind _returnvalue (`KismetSystemLibrary.K2_SetTimer` null "-IsAttacking" 0.1))
    (set `self.Timer -IsAttacking` _returnvalue)
    (if (not (`/Game/Blueprints/BP_MainChacter.IsPlayingAnimation` (`self.NPC`)))
      (set `/Game/Blueprints/BP_MainChacter.IsFire` true (`self.NPC`)))
    (else
      (set `self.IsAttacking` false)
      (`self.-FindGoal`)
      (`KismetSystemLibrary.K2_ClearAndInvalidateTimerHandle` (`self.Timer -IsAttacking`)))))

(fn `-MoveToLocation`
  (`AIController.MoveToLocation` (`self.NPC_AIController`) (`self.LocationGoal`) 0.0 true true false true null true)
  (if (<= (`KismetMathLibrary.VSize` (- (`Actor.K2_GetActorLocation` (`self.NPC`)) (`self.LocationGoal`))) 100.0)
    (`self.-FindGoal` :!label _label)
    (elif (`self.-SeeTheGoalNow`)
      (goto _label)
      (else
        (bind _returnvalue (`KismetSystemLibrary.K2_SetTimer` null "-MoveToLocation" 0.1))
        (set `self.Timer -MoveToLocation` _returnvalue)))))

(fn `-SeeTheGoalNow`
  (returns (TurnSuccesful :type Boolean))
  (bind _npc (`self.NPC`))
  (bind _goal_player (`self.Goal Player`))
  (if (`/Game/Blueprints/BP_MainChacter.isDeath` _goal_player)
    (return true)
    (else
      (bind _outhit (`KismetSystemLibrary.LineTraceSingle` (`Actor.K2_GetActorLocation` _npc) (`Actor.K2_GetActorLocation` _goal_player) "TraceTypeQuery1" false (`|MakeArray` _npc :!type "Actor Object Reference") "ForDuration"))
      (bind _goal_player_2 (`self.Goal Player`)
        (:`then`
          (if (== (`.HitActor` (`GameplayStatics.BreakHitResult` _outhit)) _goal_player_2)
            (return true)
            (else
              _)))
        (:`else`
          _))
      (return false))))

(fn `-StopToLocation`
  (`MovementComponent.StopMovementImmediately` (`Character.CharacterMovement` (`self.NPC`))))

(fn `-TurnToGoal`
  (bind _npc (`self.NPC`))
  (bind (_returnvalue_roll _returnvalue_pitch) (`KismetMathLibrary.BreakRotator` (`Actor.K2_GetActorRotation` _npc)))
  (bind _goal_player (`self.Goal Player`)
    (:`then`
      (`Actor.K2_SetActorRotation` (`self.NPC`) (`KismetMathLibrary.MakeRotator` _returnvalue_roll _returnvalue_pitch (.yaw (`KismetMathLibrary.FindLookAtRotation` (`Actor.K2_GetActorLocation` _npc) (`Actor.K2_GetActorLocation` _goal_player)))) false)
      (set `self.LocationGoal` (`Actor.K2_GetActorLocation` _goal_player)))
    (:`else`)))