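; BP_StorageActor is an interactable item actor that shows an info widget when the player comes near.
; On BeginPlay it passes its ItemInfo to the W_itemInfo widget held by a widget component.
; Static mesh overlaps with BP_PlayerCharacter toggle that component's visibility.
; Interact hides the widget and returns success, the ItemInfo and a self reference, leaving any further handling to the caller.
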(event `self.ReceiveBeginPlay`
  ;[1 1 1] SetWidget
  (bind _asw_item_info (cast `/Game/UI/Widget/W_itemInfo` (`WidgetComponent.GetUserWidgetObject` (`self.W_ItemInfo`))))
  (`/Game/UI/Widget/W_itemInfo.-SetTextItemInfo` _asw_item_info (`self.ItemInfo`)))

(event `self.StaticMesh.OnComponentBeginOverlap`
  (params (OverlappedComponent :type "PrimitiveComponent Object Reference") (OtherActor :type "Actor Object Reference") (OtherComp :type "PrimitiveComponent Object Reference") (OtherBodyIndex :type Integer) (bFromSweep :type Boolean) (SweepResult :type "HitResult Structure (by ref)"))
  (cast `/Game/Blueprints/Player/BP_PlayerCharacter` OtherActor)
  (`SceneComponent.SetVisibility` (`self.W_ItemInfo`) true false))

(event `self.StaticMesh.OnComponentEndOverlap`
  (params (OverlappedComponent :type "PrimitiveComponent Object Reference") (OtherActor :type "Actor Object Reference") (OtherComp :type "PrimitiveComponent Object Reference") (OtherBodyIndex :type Integer))
  (cast `/Game/Blueprints/Player/BP_PlayerCharacter` OtherActor)
  (`SceneComponent.SetVisibility` (`self.W_ItemInfo`) false false))

(fn `Interact`
  (returns (Succesful :type Boolean) (ItemInfo :type "/Game/Data/Struct/Str_ItemInfo Structure") (Item :type "/Game/Blueprints/Storage/BP_StorageActor Object Reference"))
  (`SceneComponent.SetVisibility` (`self.W_ItemInfo`) false false)
  (return true (`self.ItemInfo`) self))

(fn `UserConstructionScript`)