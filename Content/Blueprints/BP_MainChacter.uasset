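; BP_MainChacter is a character Blueprint with health, movement states and weapon fire, handling death for both player and NPC controllers.
; Tick sets walk speed from sprint, run and ironsight flags, and passes the target location to the current fire weapon while IsFire is set.
; Storage and health components initialize on BeginPlay, and damage feeds the health component.
; IsDeath disables player movement and input, then ragdolls player or NPC after a short timer.
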(event `self.ReceiveBeginPlay`
  ;[0.2917 0.1303 1] BeginPlay
  (`self.-Init`))

(event `self.ReceiveTick`
  (params (DeltaSeconds :type "Float (single-precision)"))
  (`|ExecutionSequence`
    (:`then_0`
      ;[1 1 1] Ironsights
      (if (`self.IsIronSights`)
        (`self.-IronSights`)
        (else
          (`self.-Sprint`))))
    (:`then_1`
      ;[1 1 1] Running
      (if (and (not (`self.IsIronSights`)) (not (`self.IsSprint`)) (`self.IsRunning`))
        (set `CharacterMovementComponent.MaxWalkSpeed` (`self.Run`) (`self.CharacterMovement`))
        (elif (not (`self.IsSprint`))
          (set `CharacterMovementComponent.MaxWalkSpeed` (`self.Walk`) (`self.CharacterMovement`)))))
    (:`then_2`
      ;[1 1 1] Weapon -IsFire
      (if (`self.IsFire`)
        (bind _weaponcurrent (`/Game/Blueprints/Components/BP_Storage_Component.WeaponCurrent` (`self.BP_Storage_Component`))
          (:`then`
            (bind _asbp_weapon_fire_actor (cast `/Game/Blueprints/Storage/Weapon/Fire/BP_WeaponFireActor` _weaponcurrent))
            (`/Game/Blueprints/Storage/Weapon/Fire/BP_WeaponFireActor.-IsFire` _asbp_weapon_fire_actor (`self.WeaponTargetLocation`)))
          (:`else`))))))

(event `self.ReceiveAnyDamage`
  (params (Damage :type "Float (single-precision)") (DamageType :type "DamageType Object Reference") (InstigatedBy :type "Controller Object Reference") (DamageCauser :type "Actor Object Reference"))
  ;[1 1 1] AnyDamage
  (`/Game/Blueprints/Components/BP_HealthComponent.-Health Change` (`self.BP_HealthComponent`) (* Damage -1.0)))

(fn `-EnableRagdoll`
  (`PrimitiveComponent.SetCollisionEnabled` (`self.CapsuleComponent`) "NoCollision")
  (`PrimitiveComponent.SetCollisionEnabled` (`self.Head Col`) "NoCollision")
  (`PrimitiveComponent.SetSimulatePhysics` (`self.Mesh`) true)
  (`PrimitiveComponent.SetCollisionEnabled` (`self.Mesh`) "QueryAndPhysics")
  (`PrimitiveComponent.SetCollisionResponseToAllChannels` (`self.Mesh`) "ECR_Block"))

(fn `-Init`
  ;[1 1 1] Storage Init
  (`/Game/Blueprints/Components/_BP_Main_component.-Init` (`self.BP_Storage_Component`))
  ;[1 1 1] Health Init
  (`/Game/Blueprints/Components/_BP_Main_component.-Init` (`self.BP_HealthComponent`)))

(fn `-IronSights`
  (if (`self.IsIronSights`)
    (set `CharacterMovementComponent.MaxWalkSpeed` (`self.Walk`) (`self.CharacterMovement`))
    (else
      (set `CharacterMovementComponent.MaxWalkSpeed` (`self.Run`) (`self.CharacterMovement`)))))

(fn `-IsDeath`
  (set `self.isDeath` true)
  (bind _asplayer_controller (cast `PlayerController` (`self.GetInstigatorController`))
    (:`then`
      (`CharacterMovementComponent.DisableMovement` (`self.CharacterMovement`))
      (`self.DisableInput` _asplayer_controller null))
    (:`CastFailed`
      (cast `/Game/Blueprints/NPC/BP_NPC_AIController` (`self.GetInstigatorController`))))
  (`KismetSystemLibrary.K2_SetTimer` null "-EnableRagdoll" 1.0))

(fn `-Sprint`
  (if (`self.IsSprint`)
    (set `CharacterMovementComponent.MaxWalkSpeed` (`self.Sprint`) (`self.CharacterMovement`))
    (else
      (set `CharacterMovementComponent.MaxWalkSpeed` (`self.Run`) (`self.CharacterMovement`)))))

(fn `UserConstructionScript`)